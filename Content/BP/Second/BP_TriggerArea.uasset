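; BP_TriggerArea is a trigger volume that lights a spotlight and reveals props when its box is overlapped.
; On any overlap it shows the referenced SpotLight's light, then the TriggerButton's bottom and sphere meshes.
; If the DiningTable's HasEat is false, it also reveals the hamburger.
; It then sets HasOpenLight, provided the references are valid, and never hides anything again.
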(event `self.Box.OnComponentBeginOverlap`
  (params (OverlappedComponent :type "PrimitiveComponent Object Reference") (OtherActor :type "Actor Object Reference") (OtherComp :type "PrimitiveComponent Object Reference") (OtherBodyIndex :type Integer) (bFromSweep :type Boolean) (SweepResult :type "HitResult Structure (by ref)"))
  (bind _diningtable (`self.diningTable`))
  (bind _spotlight (`self.SpotLight`))
  (bind _triggerbutton (`self.TriggerButton`))
  (`/Engine/EditorBlueprintResources/StandardMacros.IsValid` _spotlight
    (:`Is Valid`
      (`SceneComponent.SetVisibility` (`/Game/BP/Second/BP_SpotLight.light` _spotlight) true false)
      (`/Engine/EditorBlueprintResources/StandardMacros.IsValid` _triggerbutton
        (:`Is Valid`
          (`SceneComponent.SetVisibility` (`/Game/BP/Second/BP_Button.Button-bottom` _triggerbutton) true false)
          (`SceneComponent.SetVisibility` (`/Game/BP/Second/BP_Button.Sphere` _triggerbutton) true false)
          (if (not (`/Game/BP/Second/BP_Table.hasEat` _diningtable))
            (`/Engine/EditorBlueprintResources/StandardMacros.IsValid` _diningtable
              (:`Is Valid`
                (`SceneComponent.SetVisibility` (`/Game/BP/Second/BP_Table.HAMBURGER` _diningtable) true false))))
          (set `self.hasOpenLight` true))))))

(fn `UserConstructionScript`)