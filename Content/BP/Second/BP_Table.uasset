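; Interactive table Blueprint that lets the player eat a hamburger once, growing the third-person character.
; Box overlap toggles player input and an F-key prompt, and opens or closes a Gate on that key.
; F checks the first BP_TriggerArea's light flag and prints a warning if it is off.
; If on, it destroys the hamburger component and a Timeline lerps the character's scale up.
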(event `Key|F`
  (params (Key :type "Key Structure"))
  (:`Pressed`
    (`/Engine/EditorBlueprintResources/StandardMacros.Gate` true :!label _label
      (:`Exit`
        (if (not (`self.hasEat`))
          (bind _outactors (`GameplayStatics.GetAllActorsOfClass` "/Game/BP/Second/BP_TriggerArea.BP_TriggerArea_C"))
          (if (`/Game/BP/Second/BP_TriggerArea.hasOpenLight` (`|GetArrayItem` _outactors))
            (`ActorComponent.K2_DestroyComponent` (`self.HAMBURGER`))
            (set `self.hasEat` true)
            (bind _outactors_2 (`GameplayStatics.GetAllActorsOfClass` "/Game/ThirdPersonBP/Blueprints/ThirdPersonCharacter.ThirdPersonCharacter_C"))
            (bind (_direction _newtrack_0) (`Timeline|Timeline_0`)
              (:`Update`
                (`self.SetActorScale3D` (`|GetArrayItem` _outactors_2) (`KismetMathLibrary.Conv_DoubleToVector` (`KismetMathLibrary.Lerp` 0.8 1.5 _newtrack_0)))))
            (else
              (`KismetSystemLibrary.PrintString` "还没开灯"))))))))

(event `self.Box.OnComponentBeginOverlap`
  (params (OverlappedComponent :type "PrimitiveComponent Object Reference") (OtherActor :type "Actor Object Reference") (OtherComp :type "PrimitiveComponent Object Reference") (OtherBodyIndex :type Integer) (bFromSweep :type Boolean) (SweepResult :type "HitResult Structure (by ref)"))
  (`self.EnableInput` (`GameplayStatics.GetPlayerController` 0))
  (`/Game/BP/Second/BP_TextRender.SetText` (`self.textRender`) true "Press \"F\"")
  (goto _label :!via `Open`))

(event `self.Box.OnComponentEndOverlap`
  (params (OverlappedComponent :type "PrimitiveComponent Object Reference") (OtherActor :type "Actor Object Reference") (OtherComp :type "PrimitiveComponent Object Reference") (OtherBodyIndex :type Integer))
  (`self.DisableInput` (`GameplayStatics.GetPlayerController` 0) null)
  (`/Game/BP/Second/BP_TextRender.SetText` (`self.textRender`) false "")
  (goto _label :!via `Close`))

(fn `UserConstructionScript`)