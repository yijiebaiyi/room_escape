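; Clickable button that opens the MagicWall's portal door once the first BP_Table found reports HasEat.
; Overlapping its Box enables mouse clicks, shows a prompt and opens a Gate; leaving reverses this.
; A gated click on either button mesh scales Charactor to 0.8 and raises the door by Timeline, with Succeed blocking replays.
; If HasEat is false, it prints a Chinese "haven't eaten yet" message instead.
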(event `self.Button-bottom.OnClicked`
  (params (TouchedComponent :type "PrimitiveComponent Object Reference") (ButtonPressed :type "Key Structure"))
  (`/Engine/EditorBlueprintResources/StandardMacros.Gate` true :!label _label
    (:`Exit`
      (bind _outactors (`GameplayStatics.GetAllActorsOfClass` "/Game/BP/Second/BP_Table.BP_Table_C"))
      (if (`/Game/BP/Second/BP_Table.hasEat` (`|GetArrayItem` _outactors))
        (`self.SetActorScale3D` (`self.Charactor`) (0.8 0.8 0.8))
        (set `self.hasClicked` true)
        (if (not (`self.succeed`))
          (bind (_direction _newtrack_0) (`Timeline|Timeline_0`)
            (:`Update`
              (`SceneComponent.K2_SetRelativeLocation` (`/Game/BP/Second/BP_MagicWall.portalDoor` (`self.MagicWall`)) (`KismetMathLibrary.MakeVector` 0.0 0.0 (`KismetMathLibrary.Lerp` 0.0 500.0 _newtrack_0)) false false)
              (set `self.succeed` true))))
        (else
          (`KismetSystemLibrary.PrintString` "还没吃饭！"))))))

(event `self.Sphere.OnClicked`
  (params (TouchedComponent :type "PrimitiveComponent Object Reference") (ButtonPressed :type "Key Structure"))
  (goto _label))

(event `self.Box.OnComponentBeginOverlap`
  (params (OverlappedComponent :type "PrimitiveComponent Object Reference") (OtherActor :type "Actor Object Reference") (OtherComp :type "PrimitiveComponent Object Reference") (OtherBodyIndex :type Integer) (bFromSweep :type Boolean) (SweepResult :type "HitResult Structure (by ref)"))
  (bind _returnvalue (`GameplayStatics.GetPlayerController` 0))
  (set `PlayerController.bEnableClickEvents` true _returnvalue)
  (set `PlayerController.bShowMouseCursor` true _returnvalue)
  (`/Game/BP/Second/BP_TextRender.SetText` (`self.textRender`) true "Click it !!!!")
  (goto _label :!via `Open`))

(event `self.Box.OnComponentEndOverlap`
  (params (OverlappedComponent :type "PrimitiveComponent Object Reference") (OtherActor :type "Actor Object Reference") (OtherComp :type "PrimitiveComponent Object Reference") (OtherBodyIndex :type Integer))
  (bind _returnvalue (`GameplayStatics.GetPlayerController` 0))
  (set `PlayerController.bEnableClickEvents` false _returnvalue)
  (set `PlayerController.bShowMouseCursor` false _returnvalue)
  (`/Game/BP/Second/BP_TextRender.SetText` (`self.textRender`) false "")
  (goto _label :!via `Close`))

(fn `UserConstructionScript`)