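; Key-locked door actor that swings open and closed when the player presses E nearby while HasKey is true.
; Box overlap with the ThirdPersonCharacter enables input, opens a Gate and shows a text prompt, whose visibility is refreshed every Tick.
; A FlipFlop alternately plays and reverses a Timeline that lerps the door's yaw across 90 degrees.
; Without the key, the prompt changes to a missing-key message.
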(event `self.ReceiveTick`
  (params (DeltaSeconds :type "Float (single-precision)"))
  (`self.TextRenderVisibility` (`self.TextRender`) (`self.PromptWordVisibility`)))

(event `Key|E`
  (params (Key :type "Key Structure"))
  (:`Pressed`
    (if (`self.HasKey`)
      (`/Engine/EditorBlueprintResources/StandardMacros.Gate` true :!label _label
        (:`Exit`
          (`/Engine/EditorBlueprintResources/StandardMacros.FlipFlop`
            (:`A`
              (bind (_direction _newtrack_0) (`Timeline|Timeline_0` :!label _label_2)
                (:`Update`
                  (`SceneComponent.K2_SetRelativeRotation` (`self.Door`) (`KismetMathLibrary.MakeRotator` 0.0 0.0 (`KismetMathLibrary.Lerp` 0.0 -90.0 _newtrack_0)) false false))))
            (:`B`
              (goto _label_2 :!via `Reverse`)))))
      (else
        (`self.SetTextRenderText` (`self.TextRender`) "You don't have the key!!")))))

(event `self.Box.OnComponentBeginOverlap`
  (params (OverlappedComponent :type "PrimitiveComponent Object Reference") (OtherActor :type "Actor Object Reference") (OtherComp :type "PrimitiveComponent Object Reference") (OtherBodyIndex :type Integer) (bFromSweep :type Boolean) (SweepResult :type "HitResult Structure (by ref)"))
  (cast `/Game/ThirdPersonBP/Blueprints/ThirdPersonCharacter` OtherActor)
  (set `self.PromptWordVisibility` true)
  (`self.SetTextRenderText` (`self.TextRender`) "Press \"E\"")
  (`self.EnableInput` (`GameplayStatics.GetPlayerController` 0))
  (goto _label :!via `Open`))

(event `self.Box.OnComponentEndOverlap`
  (params (OverlappedComponent :type "PrimitiveComponent Object Reference") (OtherActor :type "Actor Object Reference") (OtherComp :type "PrimitiveComponent Object Reference") (OtherBodyIndex :type Integer))
  (cast `/Game/ThirdPersonBP/Blueprints/ThirdPersonCharacter` OtherActor)
  (set `self.PromptWordVisibility` false)
  (`self.DisableInput` (`GameplayStatics.GetPlayerController` 0))
  (goto _label :!via `Close`))

(event `TextRenderVisibility`
  (params (textRender :type "TextRenderComponent Object Reference") (visibility :type Boolean))
  (if visibility
    (`SceneComponent.SetVisibility` textRender true false)
    (else
      (`SceneComponent.SetVisibility` textRender false false))))

(event `SetTextRenderText`
  (params (TextRender :type "TextRenderComponent Object Reference") (TextContent :type Text))
  (`TextRenderComponent.K2_SetText` TextRender TextContent))

(fn `UserConstructionScript`)