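; BP_DoorKey is a key pickup that the player collects with F to flag a BP_OpenDoorByKey door as having its key.
; Box overlap by the ThirdPersonCharacter shows a text prompt, enables input and opens a gate, unless the door already has the key.
; Pressing F sets HasKey on the first door found by GetAllActorsOfClass and destroys the pickup.
; Tick applies the prompt's visibility flag every frame.
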(event `self.ReceiveTick`
  (params (DeltaSeconds :type "Float (single-precision)"))
  (bind _textrender (`self.TextRender`))
  (if (`self.TextRenderVisibility`)
    (`SceneComponent.SetVisibility` _textrender true false)
    (else
      (`SceneComponent.SetVisibility` _textrender false false))))

(event `Key|F`
  (params (Key :type "Key Structure"))
  (:`Pressed`
    (`/Engine/EditorBlueprintResources/StandardMacros.Gate` true :!label _label
      (:`Exit`
        (bind _outactors (`GameplayStatics.GetAllActorsOfClass` "/Game/BP/First/BP_OpenDoorByKey.BP_OpenDoorByKey_C"))
        (set `/Game/BP/First/BP_OpenDoorByKey.HasKey` true (`|GetArrayItem` _outactors))
        (`self.K2_DestroyActor`)
        (set `self.TextRenderVisibility` false)))))

(event `self.Box.OnComponentBeginOverlap`
  (params (OverlappedComponent :type "PrimitiveComponent Object Reference") (OtherActor :type "Actor Object Reference") (OtherComp :type "PrimitiveComponent Object Reference") (OtherBodyIndex :type Integer) (bFromSweep :type Boolean) (SweepResult :type "HitResult Structure (by ref)"))
  (cast `/Game/ThirdPersonBP/Blueprints/ThirdPersonCharacter` OtherActor)
  (bind _outactors (`GameplayStatics.GetAllActorsOfClass` "/Game/BP/First/BP_OpenDoorByKey.BP_OpenDoorByKey_C"))
  (if (not (`/Game/BP/First/BP_OpenDoorByKey.HasKey` (`|GetArrayItem` _outactors)))
    (set `self.TextRenderVisibility` true)
    (`self.EnableInput` (`GameplayStatics.GetPlayerController` 0))
    (goto _label :!via `Open`)))

(event `self.Box.OnComponentEndOverlap`
  (params (OverlappedComponent :type "PrimitiveComponent Object Reference") (OtherActor :type "Actor Object Reference") (OtherComp :type "PrimitiveComponent Object Reference") (OtherBodyIndex :type Integer))
  (cast `/Game/ThirdPersonBP/Blueprints/ThirdPersonCharacter` OtherActor)
  (set `self.TextRenderVisibility` false)
  (`self.DisableInput` (`GameplayStatics.GetPlayerController` 0))
  (goto _label :!via `Close`))

(fn `UserConstructionScript`)