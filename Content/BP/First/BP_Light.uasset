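; BP_Light is an interactable spotlight that the player switches on with the G key while standing in its trigger box.
; Box overlap by ThirdPersonCharacter toggles actor input and a gate, showing a text prompt only if the light is still off.
; Pressing G through the open gate reveals the spotlight, sets TurnOnLight and fires the passLevel custom event through a "ce" console command.
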(event `Key|G`
  (params (Key :type "Key Structure"))
  (:`Pressed`
    (`/Engine/EditorBlueprintResources/StandardMacros.Gate` true :!label _label
      (:`Exit`
        (`SceneComponent.SetVisibility` (`self.SpotLight`) true false)
        (set `self.TurnOnLight` true)
        (`KismetSystemLibrary.ExecuteConsoleCommand` "ce passLevel" null)))))

(event `self.Box.OnComponentBeginOverlap`
  (params (OverlappedComponent :type "PrimitiveComponent Object Reference") (OtherActor :type "Actor Object Reference") (OtherComp :type "PrimitiveComponent Object Reference") (OtherBodyIndex :type Integer) (bFromSweep :type Boolean) (SweepResult :type "HitResult Structure (by ref)"))
  (cast `/Game/ThirdPersonBP/Blueprints/ThirdPersonCharacter` OtherActor)
  (`self.EnableInput` (`GameplayStatics.GetPlayerController` 0))
  (if (not (`self.TurnOnLight`))
    (`SceneComponent.SetVisibility` (`self.TextRender`) true false)
    (goto _label :!via `Open`)))

(event `self.Box.OnComponentEndOverlap`
  (params (OverlappedComponent :type "PrimitiveComponent Object Reference") (OtherActor :type "Actor Object Reference") (OtherComp :type "PrimitiveComponent Object Reference") (OtherBodyIndex :type Integer))
  (cast `/Game/ThirdPersonBP/Blueprints/ThirdPersonCharacter` OtherActor)
  (`self.DisableInput` (`GameplayStatics.GetPlayerController` 0))
  (`SceneComponent.SetVisibility` (`self.TextRender`) false false)
  (goto _label :!via `Close`))

(fn `UserConstructionScript`)